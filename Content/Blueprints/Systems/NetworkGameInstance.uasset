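; Game instance that handles multiplayer session hosting, searching and joining through the Advanced Sessions nodes, and shows the main menu widget.
; Hosting creates a session with a hard-coded SERVERNAME setting, then opens ThirdPersonExampleMap as a listen server.
; A successful search stores the results and immediately joins the first one without checking for an empty list, then prints its server name.
; ShowMenuHUD creates and displays the menu only when no valid instance exists.
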(event `Search Servers`
  ;[1 1 1] Server Creation
  (`KismetArrayLibrary.Array_Clear` (`self.Found Servers`))
  (bind _results (`FindSessionsCallbackProxyAdvanced.FindSessionsAdvanced` (`GameplayStatics.GetPlayerController` 0) 999 false "AllServers")
    (:`OnSuccess`
      (set `self.Found Servers` _results)
      (`self.Join Server`))))

(event `Join Server`
  (bind _output (`|GetArrayItem` (`self.Found Servers`)))
  ;[1 1 1] Server Creation
  (`JoinSessionCallbackProxy.JoinSession` (`GameplayStatics.GetPlayerController` 0) _output
    (:`OnSuccess`
      (bind _extrasettings (`AdvancedSessionsLibrary.GetExtraSettings` _output))
      (bind _settingvalue (`AdvancedSessionsLibrary.GetSessionPropertyString` _extrasettings "SERVERNAME")
        (:`Found`
          (`KismetSystemLibrary.PrintString` _settingvalue))))))

(event `Host Session/Server`
  ;[1 1 1] Server Creation
  (`CreateSessionCallbackProxyAdvanced.CreateAdvancedSession` (`|MakeArray` (`AdvancedSessionsLibrary.MakeLiteralSessionPropertyString` "SERVERNAME" "sasha's Server")) (`GameplayStatics.GetPlayerController` 0) 999 999
    (:`OnSuccess`
      (`GameplayStatics.OpenLevel` "ThirdPersonExampleMap" true "listen"))))

(event `Show Menu HUD`
  (`/Engine/EditorBlueprintResources/StandardMacros.IsValid` (`self.Main Menu UI`)
    (:`Is Not Valid`
      (bind _returnvalue (`|CreateWidget` "/Game/UI/1_MenuUI.1_MenuUI_C" (`GameplayStatics.GetPlayerController` 0)))
      (bind _output_get (set `self.Main Menu UI` _returnvalue))
      (`UserWidget.AddToViewport` _output_get 0))))